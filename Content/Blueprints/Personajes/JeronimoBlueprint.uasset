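; Jerónimo character Blueprint for a VR experience, which talks and plays animations in response to interactions.
; Its ZonaActivacion trigger registers it as the character in range on the player's VRPawn and clears it on exit, also stopping its voice.
; Interact events play one-shot animations: Hablar restarts a stored 2D voice clip, while Pose, Simple and Conjunta silence it.
; BeginPlay sets the initial pose.
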(event OnComponentBeginOverlap(ZonaActivacion)
  (params (OverlappedComponent :type Primitive%20Component%20Object%20Reference) (OtherActor :type Actor%20Object%20Reference) (OtherComp :type Primitive%20Component%20Object%20Reference) (OtherBodyIndex :type Integer) (bFromSweep :type Boolean) (SweepResult :type Hit%20Result%20Structure%20%28by%20ref%29))
  ;[1 1 1] Eventos de Salida
  (bind _asvrpawn (Utilities|Casting|CastToVRPawn (Game|Player|GetPlayerPawn 0)))
  (Default|SetPersonajeEnRango _asvrpawn self))

(event OnComponentEndOverlap(ZonaActivacion)
  (params (OverlappedComponent :type Primitive%20Component%20Object%20Reference) (OtherActor :type Actor%20Object%20Reference) (OtherComp :type Primitive%20Component%20Object%20Reference) (OtherBodyIndex :type Integer))
  ;[1 1 1] Eventos de Salida
  (Utilities|FlowControl|Sequence
    (:then_0
      (Utilities|IsValid (Variables|Default|GetVozActual)
        (:Is%20Valid
          (Audio|Components|Audio|Stop (Variables|Default|GetVozActual)))))
    (:then_1
      (bind _asvrpawn (Utilities|Casting|CastToVRPawn (Game|Player|GetPlayerPawn 0)))
      (Default|SetPersonajeEnRango _asvrpawn))))

(event EventBeginPlay
  ;[1 1 1] Eventos de Entrada
  (Components|Animation|PlayAnimation (Variables|Default|GetSkeletalMesh) "/Game/Assets/Personajes/Jeronimo/Jeronimo_Anim_root_JerónimoPose.Jeronimo_Anim_root_JerónimoPose" false))

(event EventInteractSimple
  ;[1 1 1] Eventos de Entrada
  (Utilities|FlowControl|Sequence
    (:then_0
      (Utilities|IsValid (Variables|Default|GetVozActual)
        (:Is%20Valid
          (Audio|Components|Audio|Stop (Variables|Default|GetVozActual)))))
    (:then_1
      (Components|Animation|PlayAnimation (Variables|Default|GetSkeletalMesh) "/Game/Assets/Personajes/Jeronimo/Jeronimo_Anim_root_JéronimoSimple.Jeronimo_Anim_root_JéronimoSimple" false))))

(event EventInteractConjunta
  ;[1 1 1] Eventos de Entrada
  (Utilities|FlowControl|Sequence
    (:then_0
      (Utilities|IsValid (Variables|Default|GetVozActual)
        (:Is%20Valid
          (Audio|Components|Audio|Stop (Variables|Default|GetVozActual)))))
    (:then_1
      (Components|Animation|PlayAnimation (Variables|Default|GetSkeletalMesh) "/Game/Assets/Personajes/Jeronimo/Jeronimo_Anim_root_JéronimoConjunta.Jeronimo_Anim_root_JéronimoConjunta" false))))

(event EventInteractHablar
  ;[1 1 1] Eventos de Entrada
  (Utilities|FlowControl|Sequence
    (:then_0
      (Utilities|IsValid (Variables|Default|GetVozActual)
        (:Is%20Valid
          (Audio|Components|Audio|Stop (Variables|Default|GetVozActual))
          (bind _returnvalue (Audio|SpawnSound2D "/Game/Sonoro/ElevenLabs_Jéronimo.ElevenLabs_Jéronimo" 1.0 1.0 0.0 0))
          (Variables|Default|SetVozActual _returnvalue))
        (:Is%20Not%20Valid
          (bind _returnvalue_2 (Audio|SpawnSound2D "/Game/Sonoro/ElevenLabs_Jéronimo.ElevenLabs_Jéronimo" 1.0 1.0 0.0 0))
          (Variables|Default|SetVozActual _returnvalue_2))))
    (:then_1
      (Components|Animation|PlayAnimation (Variables|Default|GetSkeletalMesh) "/Game/Assets/Personajes/Jeronimo/Jeronimo_Anim_root_JéronimoHablar.Jeronimo_Anim_root_JéronimoHablar" false))))

(event EventInteractPose
  ;[1 1 1] Eventos de Entrada
  (Utilities|FlowControl|Sequence
    (:then_0
      (Utilities|IsValid (Variables|Default|GetVozActual)
        (:Is%20Valid
          (Audio|Components|Audio|Stop (Variables|Default|GetVozActual)))))
    (:then_1
      (Components|Animation|PlayAnimation (Variables|Default|GetSkeletalMesh) "/Game/Assets/Personajes/Jeronimo/Jeronimo_Anim_root_JerónimoPose.Jeronimo_Anim_root_JerónimoPose" false))))

(fn ConstructionScript)