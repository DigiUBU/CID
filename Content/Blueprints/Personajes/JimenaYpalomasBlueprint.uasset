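; Interactive VR character of Jimena with two pigeons, each a skeletal mesh playing one-shot animations and starting in a pose.
; An activation zone registers it with the VRPawn as the character in range, then on exit clears that and stops the voice.
; Hablar, Simple, Conjunta and Pose interaction events switch animations and stop current audio.
; Hablar also plays her 2D voice line, while Conjunta hides both pigeons.
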(event OnComponentBeginOverlap(ZonaActivacion)
  (params (OverlappedComponent :type Primitive%20Component%20Object%20Reference) (OtherActor :type Actor%20Object%20Reference) (OtherComp :type Primitive%20Component%20Object%20Reference) (OtherBodyIndex :type Integer) (bFromSweep :type Boolean) (SweepResult :type Hit%20Result%20Structure%20%28by%20ref%29))
  ;[1 1 1] Eventos de Salida
  (bind _asvrpawn (Utilities|Casting|CastToVRPawn (Game|Player|GetPlayerPawn 0)))
  (Default|SetPersonajeEnRango _asvrpawn self))

(event OnComponentEndOverlap(ZonaActivacion)
  (params (OverlappedComponent :type Primitive%20Component%20Object%20Reference) (OtherActor :type Actor%20Object%20Reference) (OtherComp :type Primitive%20Component%20Object%20Reference) (OtherBodyIndex :type Integer))
  ;[1 1 1] Eventos de Salida
  (Utilities|FlowControl|Sequence
    (:then_0
      (Utilities|IsValid (Variables|Default|GetVozActual)
        (:Is%20Valid
          (Audio|Components|Audio|Stop (Variables|Default|GetVozActual)))))
    (:then_1
      (bind _asvrpawn (Utilities|Casting|CastToVRPawn (Game|Player|GetPlayerPawn 0)))
      (Default|SetPersonajeEnRango _asvrpawn))))

(event EventBeginPlay
  ;[1 1 1] Eventos de Entrada
  (Utilities|FlowControl|Sequence
    (:then_0
      (Components|Animation|PlayAnimation (Variables|Default|GetSkeletalMesh) "/Game/Assets/Personajes/Jimena/Jimena_Anim_root_JimenaPose.Jimena_Anim_root_JimenaPose" false))
    (:then_1
      (Components|Animation|PlayAnimation (Variables|Default|GetSkeletalMeshPaloma1) "/Game/Assets/Palomas/Paloma1/Paloma1_Anim_RootPaloma1_Paloma1Pose.Paloma1_Anim_RootPaloma1_Paloma1Pose" false))
    (:then_2
      (Components|Animation|PlayAnimation (Variables|Default|GetSkeletalMeshPaloma2) "/Game/Assets/Palomas/Paloma2/Paloma2_Anim_RootPaloma2_Paloma2Pose.Paloma2_Anim_RootPaloma2_Paloma2Pose" false))))

(event EventInteractSimple
  ;[1 1 1] Eventos de Entrada
  (Utilities|FlowControl|Sequence
    (:then_0
      (Utilities|IsValid (Variables|Default|GetVozActual)
        (:Is%20Valid
          (Audio|Components|Audio|Stop (Variables|Default|GetVozActual)))))
    (:then_1
      (Components|Animation|PlayAnimation (Variables|Default|GetSkeletalMesh) "/Game/Assets/Personajes/Jimena/Jimena_Anim_root_JimenaSimple.Jimena_Anim_root_JimenaSimple" false))
    (:then_2
      (Rendering|SetVisibility (Variables|Default|GetSkeletalMeshPaloma1) true false)
      (Components|Animation|PlayAnimation (Variables|Default|GetSkeletalMeshPaloma1) "/Game/Assets/Palomas/Paloma1/Paloma1_Anim_RootPaloma1_Paloma1Simple.Paloma1_Anim_RootPaloma1_Paloma1Simple" false))
    (:then_3
      (Rendering|SetVisibility (Variables|Default|GetSkeletalMeshPaloma2) true false)
      (Components|Animation|PlayAnimation (Variables|Default|GetSkeletalMeshPaloma2) "/Game/Assets/Palomas/Paloma2/Paloma2_Anim_RootPaloma2_Paloma2Simple.Paloma2_Anim_RootPaloma2_Paloma2Simple" false))))

(event EventInteractConjunta
  ;[1 1 1] Eventos de Entrada
  (Utilities|FlowControl|Sequence
    (:then_0
      (Utilities|IsValid (Variables|Default|GetVozActual)
        (:Is%20Valid
          (Audio|Components|Audio|Stop (Variables|Default|GetVozActual)))))
    (:then_1
      (Components|Animation|PlayAnimation (Variables|Default|GetSkeletalMesh) "/Game/Assets/Personajes/Jimena/Jimena_Anim_root_JimenaConjunta.Jimena_Anim_root_JimenaConjunta" false))
    (:then_2
      (Rendering|SetVisibility (Variables|Default|GetSkeletalMeshPaloma1) false false))
    (:then_3
      (Rendering|SetVisibility (Variables|Default|GetSkeletalMeshPaloma2) false false))))

(event EventInteractPose
  ;[1 1 1] Eventos de Entrada
  (Utilities|FlowControl|Sequence
    (:then_0
      (Utilities|IsValid (Variables|Default|GetVozActual)
        (:Is%20Valid
          (Audio|Components|Audio|Stop (Variables|Default|GetVozActual)))))
    (:then_1
      (Components|Animation|PlayAnimation (Variables|Default|GetSkeletalMesh) "/Game/Assets/Personajes/Jimena/Jimena_Anim_root_JimenaPose.Jimena_Anim_root_JimenaPose" false))
    (:then_2
      (Rendering|SetVisibility (Variables|Default|GetSkeletalMeshPaloma1) true false)
      (Components|Animation|PlayAnimation (Variables|Default|GetSkeletalMeshPaloma1) "/Game/Assets/Palomas/Paloma1/Paloma1_Anim_RootPaloma1_Paloma1Pose.Paloma1_Anim_RootPaloma1_Paloma1Pose" false))
    (:then_3
      (Rendering|SetVisibility (Variables|Default|GetSkeletalMeshPaloma2) true false)
      (Components|Animation|PlayAnimation (Variables|Default|GetSkeletalMeshPaloma2) "/Game/Assets/Palomas/Paloma2/Paloma2_Anim_RootPaloma2_Paloma2Pose.Paloma2_Anim_RootPaloma2_Paloma2Pose" false))))

(event EventInteractHablar
  ;[1 1 1] Eventos de Entrada
  (Utilities|FlowControl|Sequence
    (:then_0
      (Utilities|IsValid (Variables|Default|GetVozActual)
        (:Is%20Valid
          (Audio|Components|Audio|Stop (Variables|Default|GetVozActual))
          (bind _returnvalue (Audio|SpawnSound2D "/Game/Sonoro/ElevenLabs_Jimena.ElevenLabs_Jimena" 1.0 1.0 0.0 0))
          (Variables|Default|SetVozActual _returnvalue))
        (:Is%20Not%20Valid
          (bind _returnvalue_2 (Audio|SpawnSound2D "/Game/Sonoro/ElevenLabs_Jimena.ElevenLabs_Jimena" 1.0 1.0 0.0 0))
          (Variables|Default|SetVozActual _returnvalue_2))))
    (:then_1
      (Components|Animation|PlayAnimation (Variables|Default|GetSkeletalMesh) "/Game/Assets/Personajes/Jimena/Jimena_Anim_root_JimenaHablar.Jimena_Anim_root_JimenaHablar" false))
    (:then_2
      (Rendering|SetVisibility (Variables|Default|GetSkeletalMeshPaloma1) true false)
      (Components|Animation|PlayAnimation (Variables|Default|GetSkeletalMeshPaloma1) "/Game/Assets/Palomas/Paloma1/Paloma1_Anim_RootPaloma1_Paloma1Pose.Paloma1_Anim_RootPaloma1_Paloma1Pose" false))
    (:then_3
      (Rendering|SetVisibility (Variables|Default|GetSkeletalMeshPaloma2) true false)
      (Components|Animation|PlayAnimation (Variables|Default|GetSkeletalMeshPaloma2) "/Game/Assets/Palomas/Paloma2/Paloma2_Anim_RootPaloma2_Paloma2Pose.Paloma2_Anim_RootPaloma2_Paloma2Pose" false))))

(fn ConstructionScript)